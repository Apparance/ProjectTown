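; Base Blueprint for themeable smart objects in a town game, supplying shared theme, seed and size accessors.
; SetTheme stores the theme and calls OnThemeChange, an empty hook for derived classes to rebuild; SyncTheme pulls the global theme from BP_TownGameMode.
; GetSeed lazily generates and caches a random seed, and GetSize derives a 2D footprint from the first frame parameter.
; BeginPlay makes the root component movable.
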(event EventBeginPlay
  (Transformation|SetMobility (Variables|Transformation|GetRootComponent) "Movable"))

(event Collision|EventActorBeginOverlap
  (params (OtherActor :type Actor%20Object%20Reference)))

(event EventTick
  (params (DeltaSeconds :type Float%20%28single-precision%29)))

(event EventSetTheme
  (params (Theme :type Integer))
  (Variables|Default|SetTheme Theme)
  (CallFunction|OnThemeChange) ; Get derived to rebuild
)

(fn ConstructionScript)

(fn OnThemeChange)

(fn SyncTheme
  ;[0 0 0] Apply Global Theme
  (bind _asbp_town_game_mode (Utilities|Casting|CastToBP_TownGameMode (Game|GetGameMode)))
  (CallFunction|SetTheme (Variables|/Game/Scripts/BP_TownGameMode.BP_TownGameMode_C|GetTheme _asbp_town_game_mode)))

(fn GetSeed
  ;[0 0 0] Init on demand
  (if (== (Variables|Default|GetSeed) 0)
    (Variables|Default|SetSeed (Math|Random|RandomInteger 2000000000)))
  (return (Variables|Default|GetSeed)))

(fn GetSize
  (bind _returnvalue (Class|ApparanceBlueprintLibrary|GetCurrentParameters self))
  (bind _returnvalue_2 (Class|ApparanceBlueprintLibrary|GetFrameParameter _returnvalue))
  (return (Math|Vector2D|MakeVector2D (.X (Math|Vector|BreakVector (Class|ApparanceBlueprintLibrary|GetFrameSize _returnvalue_2))) (.Y (Math|Vector|BreakVector (Class|ApparanceBlueprintLibrary|GetFrameSize _returnvalue_2))))))

(fn GetTheme
  (return (Variables|Default|GetTheme)))