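; BP_ToolTray is a tray actor that holds spawned tools and shows them, along with its own UI, through a scene capture camera.
; When generation completes, it recursively gathers its attached actors, adds itself, and sets that list as the CaptureCamera's ShowOnlyActors.
; It then rebuilds its Tools list from the captured actors that implement BI_Tool.
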(event EventBeginPlay)

(event Collision|EventActorBeginOverlap
  (params (OtherActor :type Actor%20Object%20Reference)))

(event EventTick
  (params (DeltaSeconds :type Float%20%28single-precision%29)))

(event EventGenerationComplete
  (Utilities|FlowControl|Sequence
    (:then_0
      ;[0 0 0] Ensure All spawned tools are included in capture
      (bind _output_get (Variables|Default|SetCapture%20Actors (Actor|GetAttachedActors true true)))
      (Utilities|Array|Add _output_get self) ; Ensure ourself is captured too\n(we have UI too)
      (Variables|/Script/Engine.SceneCaptureComponent|SetShowOnlyActors (Variables|/Script/Engine.SceneCapture2D|GetCaptureComponent2D (Variables|Default|GetCapture%20Camera)) (Variables|Default|GetCapture%20Actors)))
    (:then_1
      ;[0 0 0] Gather a list of Tools
      (Utilities|Array|Clear (Variables|Default|GetTools))
      (for _array_element (Variables|Default|GetCapture%20Actors)
        (bind _asbi_tool (Utilities|Casting|CastToBI_Tool _array_element))
        (Utilities|Array|Add (Variables|Default|GetTools) _asbi_tool)))))

(fn ConstructionScript)