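; House preset Blueprint that drives an Apparance procedural entity through a Theme value and a seed.
; Theme changes, and internal theme sets with a non-zero value, rebuild the entity with that theme and the current seed, then print the seed for debugging.
; GetTheme reads the theme back from the entity's current parameters by index.
; Theme-change and BeginPlay events also call their parent implementations.
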(event Collision|EventActorBeginOverlap
  (params (OtherActor :type Actor%20Object%20Reference)))

(event EventTick
  (params (DeltaSeconds :type Float%20%28single-precision%29)))

(event EventBeginPlay
  (|CallParentFunction))

(fn ConstructionScript)

(fn SetThemeInternal
  (params (Theme :type Integer))
  (bind _seed (CallFunction|GetSeed))
  (if (!= 0 Theme) ; Do anything?
    (|ApparanceRebuildNode Theme _seed)
    (Development|PrintText (Utilities|Text|FormatText "SEED = {0} (set theme internal)" _seed))))

(fn OnThemeChange
  (bind _seed (CallFunction|GetSeed))
  (|CallParentFunction)
  (|ApparanceRebuildNode (Variables|Default|GetTheme) _seed)
  (Development|PrintText (Utilities|Text|FormatText "SEED = {0} (on theme changed)" _seed)))

(fn GetTheme
  (bind _returnvalue (Class|ApparanceBlueprintLibrary|GetCurrentParameters self))
  (bind _returnvalue_2 (Class|ApparanceBlueprintLibrary|GetIntegerParameter _returnvalue 1)) ; Get current Theme value
  (return _returnvalue_2))