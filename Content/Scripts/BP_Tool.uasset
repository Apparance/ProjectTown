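; BP_Tool is a base tool actor with default placement behaviour, built on Apparance procedural entities with a child Rectangle that receives its parameters after generation.
; Highlight and Select combine into state flags that rebuild both visuals, and Select also toggles a gate that spins the tool each tick.
; Activate spawns SpawnClass at the target position and applies the town game mode's theme.
; Getter functions supply help text, hover text and default targeting answers.
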(event EventBeginPlay)

(event Collision|EventActorBeginOverlap
  (params (OtherActor :type Actor%20Object%20Reference)))

(event EventTick
  (params (DeltaSeconds :type Float%20%28single-precision%29))
  ;[0 0 0] Default Behaviour: Base Rotation when Tool Selected
  (Utilities|FlowControl|Gate true
    (:Exit
      (Transformation|AddActorLocalRotation "0.000000,0.400000,0.000000" false false))))

(event EventHighlight
  (params (Enable :type Boolean))
  (bind _output_get (Variables|Default|SetIs%20Highlighted Enable))
  (CallFunction|ApplyState _output_get (stale EventSelect _output_get))
  (Default|ApplyState (Variables|Default|GetBP%20Tool%20Rectangle) _output_get (stale EventSelect _output_get)) ; Also Update the child Rectangle
)

(event EventSelect
  (params (Enable :type Boolean))
  (Utilities|FlowControl|Sequence
    (:then_0
      (bind _output_get (Variables|Default|SetIs%20Selected Enable))
      (CallFunction|ApplyState (stale EventHighlight _output_get) _output_get)
      (Default|ApplyState (Variables|Default|GetBP%20Tool%20Rectangle) (stale EventHighlight _output_get) _output_get) ; Also Update the child Rectangle
    )
    (:then_1
      ;[0 0 0] Default Behaviour: Base Rotation when Tool Selected
      (Utilities|FlowControl|Gate true) ; enters at Toggle
    )))

(event EventActivate
  (params (Target%20Ground%20Pos :type Vector :default "0, 0, 0") (Target%20Object :type BI%20Smart%20Object%20Interface))
  ;[0 0 0] Default Behaviour: Place Object
  (bind _asactor (Utilities|Casting|CastToActorClass (Variables|Default|GetSpawn%20Class)))
  (bind _returnvalue (Game|SpawnActorfromClass _asactor (Math|Transform|MakeTransform Target%20Ground%20Pos) "AlwaysSpawn" "MultiplyWithRoot" 0 0))
  (bind _asbi_themed (Utilities|Casting|CastToBI_Themed _returnvalue))
  (bind _asbp_town_game_mode (Utilities|Casting|CastToBP_TownGameMode (Game|GetGameMode)))
  (Default|SetTheme _asbi_themed (Variables|/Game/Scripts/BP_TownGameMode.BP_TownGameMode_C|GetTheme _asbp_town_game_mode)))

(event EventGenerationComplete
  ;[0 0 0] When Tool is properly Spawned...
  (if (not (Variables|Default|GetInitialised))
    ;[0 0 0] Grab Rectangle Ref
    (bind _asbp_tool_rectangle (Utilities|Casting|CastToBP_Tool_Rectangle (Variables|/Script/Engine.ChildActorComponent|GetChildActor (Variables|Default|GetBP_Tool_Rectangle))))
    (Variables|Default|SetBP%20Tool%20Rectangle _asbp_tool_rectangle)
    ;[0 0 0] Pass this Tool's initialised Parameters through to the Rectangle Apparance Entity for colours
    (bind _returnvalue (Class|ApparanceBlueprintLibrary|GetCurrentParameters self))
    (|ApparanceRebuildNode (Variables|Default|GetBP%20Tool%20Rectangle) _returnvalue)
    (Variables|Default|SetInitialised true)))

(fn ConstructionScript)

(fn ApplyState
  (params (IsHighlighted :type Boolean) (IsSelected :type Boolean))
  (|ApparanceRebuildNode (Class|KismetMathLibrary|OrIntInt (Math|Integer|SelectInt 1 0 IsHighlighted) (Math|Integer|SelectInt 2 0 IsSelected))))

(fn GetHelpText
  (return (Variables|Default|GetTool%20Help%20Text)))

(fn GetHighlightType
  (return 0))

(fn GetHoverText
  (return (Variables|Default|GetButton%20Hover%20Text)))

(fn WantGroundTarget
  (return false))

(fn WantInstantAction
  (return false))

(fn WantObjectTarget
  (return false))