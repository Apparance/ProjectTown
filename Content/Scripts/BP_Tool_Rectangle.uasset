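; BP_Tool_Rectangle is a child-actor part of a BP_Tool that relays highlight and selection to its parent tool.
; Highlight and Select apply one flag as both highlighted and selected state to itself and the parent, and Select also forwards the event.
; ApplyState packs both states into bit flags for an Apparance rebuild.
; Construction makes root rotation absolute, and the tool query functions return empty or false defaults.
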(event EventBeginPlay
  (bind _asbp_tool (Utilities|Casting|CastToBP_Tool (Actor|GetParentActor)))
  (Variables|Default|SetBP%20Tool _asbp_tool))

(event Collision|EventActorBeginOverlap
  (params (OtherActor :type Actor%20Object%20Reference)))

(event EventTick
  (params (DeltaSeconds :type Float%20%28single-precision%29)))

(event EventHighlight
  (params (Enable :type Boolean))
  ;[0.03551 0.2865 0.03515] Apply Highlight/Selection State, also apply to parent Tool and Select Event passed back
  (CallFunction|ApplyState Enable (stale EventSelect Enable))
  (Default|ApplyState (Variables|Default|GetBP%20Tool) Enable (stale EventSelect Enable)))

(event EventSelect
  (params (Enable :type Boolean))
  (bind _bp_tool (Variables|Default|GetBP%20Tool))
  ;[0.03551 0.2865 0.03515] Apply Highlight/Selection State, also apply to parent Tool and Select Event passed back
  (Utilities|FlowControl|Sequence
    (:then_0
      (CallFunction|ApplyState (stale EventHighlight Enable) Enable)
      (Default|ApplyState _bp_tool (stale EventHighlight Enable) Enable))
    (:then_1
      (Default|Select _bp_tool Enable))))

(fn ConstructionScript
  (Transformation|SetAbsolute (Variables|Transformation|GetRootComponent) false true false))

(fn ApplyState
  (params (IsHighlighted :type Boolean) (IsSelected :type Boolean))
  (|ApparanceRebuildNode (Class|KismetMathLibrary|OrIntInt (Math|Integer|SelectInt 1 0 IsHighlighted) (Math|Integer|SelectInt 2 0 IsSelected))))

(fn GetHelpText
  (return ""))

(fn GetHighlightType
  (return 0))

(fn GetHoverText
  (return ""))

(fn WantGroundTarget
  (return false))

(fn WantInstantAction
  (return false))

(fn WantObjectTarget
  (return false))